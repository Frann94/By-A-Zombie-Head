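; BP_Zombie is an enemy character that walks to a gate destination, then runs after the player and attacks in melee.
; AIMoveTo, pawn sensing and capsule overlaps with "Ally" actors drive a self-repeating chase and attack loop.
; The attack montage notify messages an overlapping BP_Gate and sphere-checks a hitbox to damage the player character.
; Damage plays a reaction montage; death ragdolls the mesh, swaps the sound and notifies BP_GameMode.
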(event `self.ReceiveBeginPlay`
  (`self.Move to Gate`))

(event `Move to Gate`
  (`|AIMoveTo` self (`self.GateDestination`) null
    (:`OnSuccess`
      _)
    (:`OnFail`
      _))
  (`self.Follow Player`))

(event `self.ReceiveAnyDamage`
  (params (Damage :type "Float (single-precision)") (DamageType :type "DamageType Object Reference") (InstigatedBy :type "Controller Object Reference") (DamageCauser :type "Actor Object Reference"))
  (bind _health (`self.Health`))
  (`|PlayMontage` (`self.Mesh`) "/Game/Characters/Zombie/Animation/Reaction_Montage.Reaction_Montage"
    (:`then`
      (if (> _health 0.0)
        (set `self.Health` (- _health Damage))
        (`self.Follow Player`)
        (if (<= (`self.Health`) 0.0)
          (`self.Death`))))
    (:`OnCompleted`
      (if (`self.IsOverLapping?`)
        (`KismetSystemLibrary.Delay` 0.2)
        (`self.Attack`)
        (else
          (`self.Follow Player`))))))

(event `Death`
  (bind _mesh (`self.Mesh`))
  (`PrimitiveComponent.SetCollisionEnabled` _mesh "QueryAndPhysics")
  (`PrimitiveComponent.SetSimulatePhysics` _mesh true)
  (`SkeletalMeshComponent.SetPhysicsBlendWeight` _mesh 1.0)
  (`PrimitiveComponent.SetCollisionEnabled` (`self.CapsuleComponent`) "NoCollision")
  (`AudioComponent.SetSound` (`self.Idle/Walk`) "/Game/_Main/SoundFX/zombie_death.zombie_death")
  (bind _asbp_game_mode (cast `/Game/_Main/GameMode/BP_GameMode` (`GameplayStatics.GetGameMode`)))
  (`/Game/_Main/GameMode/BP_GameMode.Enemy Killed` _asbp_game_mode))

(event `self.CapsuleComponent.OnComponentBeginOverlap`
  (params (OverlappedComponent :type "PrimitiveComponent Object Reference") (OtherActor :type "Actor Object Reference") (OtherComp :type "PrimitiveComponent Object Reference") (OtherBodyIndex :type Integer) (bFromSweep :type Boolean) (SweepResult :type "HitResult Structure (by ref)"))
  (if (`self.ActorHasTag` OtherActor "Ally")
    (set `self.IsOverLapping?` true)
    (`self.Attack`)))

(event `self.CapsuleComponent.OnComponentEndOverlap`
  (params (OverlappedComponent :type "PrimitiveComponent Object Reference") (OtherActor :type "Actor Object Reference") (OtherComp :type "PrimitiveComponent Object Reference") (OtherBodyIndex :type Integer))
  (set `self.IsOverLapping?` false)
  (`self.Follow Player`))

(event `Attack`
  (`|PlayMontage` (`self.Mesh`) "/Game/Characters/Zombie/Animation/Zombie_Attack_Montage.Zombie_Attack_Montage"
    (:`OnCompleted`
      (if (`self.IsOverLapping?`)
        (`KismetSystemLibrary.Delay` 0.2)
        (`self.Attack`)
        (else
          (`KismetSystemLibrary.Delay` 0.2)
          (`self.Follow Player`))))
    (:`OnNotifyBegin`
      (message `/Game/_Main/Interfaces/BPI_DestroyGate.DestroyGate` (`|GetArrayItem` (`self.GetOverlappingActors` "/Game/_Main/Gate/BP_Gate.BP_Gate_C")))
      (bind (_outactors _returnvalue) (`KismetSystemLibrary.SphereOverlapActors` (`SceneComponent.K2_GetComponentLocation` (`self.HitBoxLocation`)) 40.0 (`|MakeArray` "ObjectTypeQuery3" :!type "EObjectTypeQuery Enum") "/Game/ThirdPerson/Blueprints/BP_ThirdPersonCharacter.BP_ThirdPersonCharacter_C" (`|MakeArray` self :!type "Actor Object Reference")))
      (if _returnvalue
        (for _array_element _outactors
          (`GameplayStatics.ApplyDamage` _array_element 10.0 (`self.GetController`) self "/Script/Engine.DamageType"))))))

(event `Follow Player`
  (set `CharacterMovementComponent.MaxWalkSpeed` 400.0 (`self.CharacterMovement`))
  (`|AIMoveTo` self (0.0 0.0 0.0) (`GameplayStatics.GetPlayerController` 0) 1.0
    (:`OnSuccess`
      (`/Engine/EditorBlueprintResources/StandardMacros.DoOnce` false :!label _label
        (:`Completed`
          (`self.Attack`)
          (`KismetSystemLibrary.Delay` 2.0)
          (`|ExecutionSequence`
            (:`then_0`
              (goto _label :!via `Reset`))
            (:`then_1`
              (`self.Follow Player`))))))
    (:`OnFail`
      (`self.Follow Player`))))

(event `self.PawnSensing.OnSeePawn`
  (params (Pawn :type "Pawn Object Reference"))
  (`self.Follow Player`))

(fn `UserConstructionScript`)