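; BP_Gate is a gate actor that can be progressively knocked over or repaired.
; DestroyGate raises GateAngle and adds it to the roll with a hit sound until a threshold, then a timeline tips it toward 90 degrees with a falling sound.
; Delayed calls during the fall disable collision on both meshes and the box.
; RepairGate lowers GateAngle and subtracts it from the roll while it stays above zero.
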(event `/Game/_Main/Interfaces/BPI_DestroyGate.DestroyGate`
  (bind (_returnvalue_roll _returnvalue_pitch _returnvalue_yaw) (`KismetMathLibrary.BreakRotator` (`self.K2_GetActorRotation`)))
  (bind (_returnvalue_roll_2 _returnvalue_pitch_2 _returnvalue_yaw_2) (`KismetMathLibrary.BreakRotator` (`self.K2_GetActorRotation`)))
  (if (< (`self.Gate Angle`) 2.0)
    (bind _output_get (set `self.Gate Angle` (+ (`self.Gate Angle`) 0.1)))
    (`self.K2_SetActorRotation` (`KismetMathLibrary.MakeRotator` (+ _output_get _returnvalue_roll) _returnvalue_pitch _returnvalue_yaw))
    (`GameplayStatics.PlaySoundAtLocation` "/Game/_Main/SoundFX/gate_hit.gate_hit" (`self.Location`) (struct) 0.5 1.0 0.0 null null null null)
    (else
      (`|ExecutionSequence`
        (:`then_0`
          (`KismetSystemLibrary.Delay` 0.2)
          (bind (_direction _newtrack_0) (`Timeline|Gate Falling Timeline`)
            (:`Update`
              (`self.K2_SetActorRotation` (`KismetMathLibrary.MakeRotator` (`KismetMathLibrary.MapRangeClamped` _newtrack_0 0.0 90.0 _returnvalue_roll_2 90.0) _returnvalue_pitch_2 _returnvalue_yaw_2))
              (`KismetSystemLibrary.Delay` 0.5)
              (`PrimitiveComponent.SetCollisionEnabled` (`self.GateMesh`) "NoCollision")
              (`PrimitiveComponent.SetCollisionEnabled` (`self.Box`) "NoCollision")
              (`PrimitiveComponent.SetCollisionEnabled` (`self.GateMesh1`) "NoCollision"))))
        (:`then_1`
          (`GameplayStatics.PlaySoundAtLocation` "/Game/_Main/SoundFX/gate_falling.gate_falling" (`self.Location`) (struct) 0.5 1.0 0.0 null null null null))))))

(event `/Game/_Main/Interfaces/BPI_RepairGate.RepairGate`
  (bind (_returnvalue_roll _returnvalue_pitch _returnvalue_yaw) (`KismetMathLibrary.BreakRotator` (`self.K2_GetActorRotation`)))
  (bind _returnvalue (- (`self.Gate Angle`) 0.1))
  (if (not (<= _returnvalue 0.0))
    (bind _output_get (set `self.Gate Angle` _returnvalue))
    (`self.K2_SetActorRotation` (`KismetMathLibrary.MakeRotator` (- _returnvalue_roll _output_get) _returnvalue_pitch _returnvalue_yaw))
    (`GameplayStatics.PlaySoundAtLocation` "/Game/_Main/SoundFX/gate_hit.gate_hit" (`self.Location`) (struct) 0.5 1.0 0.0 null null null null)))

(fn `UserConstructionScript`)