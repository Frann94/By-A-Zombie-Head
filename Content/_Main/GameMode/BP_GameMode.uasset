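; Game mode that runs a wave-based zombie survival loop and toggles a pause menu.
; Each wave sounds an alarm, waits while a warning widget shows, then spawns three zombies per wave number at a single spawn transform.
; Kill notifications decrement a remaining count that triggers the next wave at zero.
; A free mode freezes existing zombies, resets the wave counter and stops wave progression until restart.
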(event `self.ReceiveBeginPlay`
  (`|ExecutionSequence`
    (:`then_0`
      (`WidgetBlueprintLibrary.SetInputMode_GameOnly` (`GameplayStatics.GetPlayerController` 0))
      (bind _returnvalue (`|CreateWidget` "/Game/_Main/HUD/UI_WaveWarning.UI_WaveWarning_C"))
      (bind _output_get (set `self.WaveWarningWidget` _returnvalue))
      (`UserWidget.AddToViewport` _output_get 0)
      (`self.Start Game`))
    (:`then_2`
      (bind _returnvalue_2 (`|CreateWidget` "/Game/_Main/HUD/UI_InGameMenu.UI_InGameMenu_C"))
      (bind _output_get_2 (set `self.GameMenuWidget` _returnvalue_2))
      (`Widget.SetVisibility` _output_get_2 "Hidden")
      (`UserWidget.AddToViewport` _output_get_2 0))))

(event `Start Game`
  (bind _spawn_location_location (`KismetMathLibrary.BreakTransform` (`self.Spawn Location`)))
  (`GameplayStatics.PlaySoundAtLocation` "/Game/Interface_And_Item_Sounds/Cues/Futuristic_Alarm_01_Cue.Futuristic_Alarm_01_Cue" _spawn_location_location (struct) 0.08 1.0 5.0 null null null null)
  (`KismetSystemLibrary.Delay` 5.0)
  (`Widget.SetVisibility` (`self.WaveWarningWidget`) "Hidden")
  (`self.Spawn Enemies`))

(event `Spawn Enemies`
  (bind _output_get (set `self.Total Enemies` (* (`self.Current Wave`) 3)))
  (set `self.Remaining Enemies` _output_get)
  (for _index (range (+ _output_get 1))
    (if (!= _index (`self.Total Enemies`))
      (`|SpawnActorFromClass` "/Game/Characters/Zombie/BP_Zombie.BP_Zombie_C" (`self.Spawn Location`) "AdjustIfPossibleButAlwaysSpawn" "MultiplyWithRoot" null null)
      (else
        (break)))))

(event `Enemy Killed`
  (bind _result (`/Engine/EditorBlueprintResources/StandardMacros.DecrementInt` (`self.Remaining Enemies`))
    (:`  `
      (if (and (== _result 0) (not (`self.FreeMode?`)))
        (`self.Wave Increment`)))))

(event `Wave Increment`
  (bind _spawn_location_location (`KismetMathLibrary.BreakTransform` (`self.Spawn Location`)))
  (`/Engine/EditorBlueprintResources/StandardMacros.IncrementInt` (`self.Current Wave`)
    (:`  `
      (`Widget.SetVisibility` (`self.WaveWarningWidget`) "Visible")
      (`GameplayStatics.PlaySoundAtLocation` "/Game/Interface_And_Item_Sounds/Cues/Futuristic_Alarm_01_Cue.Futuristic_Alarm_01_Cue" _spawn_location_location (struct) 0.08 1.0 5.0 null null null null)
      (`KismetSystemLibrary.Delay` 10.0)
      (`Widget.SetVisibility` (`self.WaveWarningWidget`) "Hidden")
      (`self.Spawn Enemies`))))

(event `GameMenu`
  (bind _returnvalue (`GameplayStatics.GetPlayerController` 0))
  (bind _gamemenuwidget (`self.GameMenuWidget`))
  (if (`GameplayStatics.IsGamePaused`)
    (`GameplayStatics.SetGamePaused` false)
    (`Widget.SetVisibility` _gamemenuwidget "Hidden")
    (set `PlayerController.bShowMouseCursor` false _returnvalue)
    (`WidgetBlueprintLibrary.SetInputMode_GameOnly` _returnvalue)
    (else
      (`GameplayStatics.SetGamePaused` true)
      (`Widget.SetVisibility` _gamemenuwidget "Visible")
      (`WidgetBlueprintLibrary.SetInputMode_GameAndUIEx` _returnvalue _gamemenuwidget)
      (set `PlayerController.bShowMouseCursor` true _returnvalue))))

(event `Free Mode`
  (`|ExecutionSequence`
    (:`then_0`
      (bind _outactors (`GameplayStatics.GetAllActorsOfClass` "/Game/Characters/Zombie/BP_Zombie.BP_Zombie_C"))
      (for _array_element _outactors
        (`ActorComponent.Deactivate` (`Character.CharacterMovement` _array_element))
        (`AudioComponent.SetPaused` (`/Game/Characters/Zombie/BP_Zombie.Idle/Walk` _array_element) true)))
    (:`then_1`
      (set `self.Current Wave` 0))
    (:`then_2`
      (if (`self.FreeMode?`)
        (`KismetSystemLibrary.PrintText` "TO DISABLE FREEMODE RESTART GAME" true true (struct :`G` 0.284335 :`B` 1.0 :`A` 1.0) 5.0)
        (else
          (set `self.FreeMode?` true))))))

(fn `UserConstructionScript`)